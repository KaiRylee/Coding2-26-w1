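; BP_Door is a locked door in the stealth game that opens by destroying itself when the player has a key.
; On box overlap, it casts to BP_FirstPersonCharacter, then spends one KeyCount, shows WBP_DoorOpened and destroys the actor.
; Without a key, it shows WBP_FindAKey and removes it after a short delay.
; The construction script sets the SMDoor mesh from BookLook.
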(event `self.Box collision.OnComponentBeginOverlap`
  (params (OverlappedComponent :type "PrimitiveComponent Object Reference") (OtherActor :type "Actor Object Reference") (OtherComp :type "PrimitiveComponent Object Reference") (OtherBodyIndex :type Integer) (bFromSweep :type Boolean) (SweepResult :type "HitResult Structure (by ref)"))
  (bind _asbp_first_person_character (cast `/Game/FirstPerson/Blueprints/BP_FirstPersonCharacter` OtherActor))
  (bind _key_count (`/Game/FirstPerson/Blueprints/BP_FirstPersonCharacter.Key Count` _asbp_first_person_character))
  (if (> _key_count 0)
    (set `/Game/FirstPerson/Blueprints/BP_FirstPersonCharacter.Key Count` (- _key_count 1) _asbp_first_person_character)
    (`self.SetActorHiddenInGame` false)
    (bind _returnvalue (`|CreateWidget` "/Game/Emma/MenuStuff/Main/WBP_DoorOpened.WBP_DoorOpened_C"))
    (`UserWidget.AddToViewport` _returnvalue 0)
    (`self.K2_DestroyActor`)
    (else
      (bind _returnvalue_2 (`|CreateWidget` "/Game/Emma/MenuStuff/Main/WBP_FindAKey.WBP_FindAKey_C"))
      (`UserWidget.AddToViewport` _returnvalue_2 0)
      (`KismetSystemLibrary.Delay` 3.0)
      (`Widget.RemoveFromParent` _returnvalue_2))))

(fn `UserConstructionScript`
  (`StaticMeshComponent.SetStaticMesh` (`self.SM_Door`) (`self.BookLook`)))