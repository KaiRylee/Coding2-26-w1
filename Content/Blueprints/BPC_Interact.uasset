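; Player interaction component for BP_FirstPersonCharacter that handles picking up, using, dropping and swapping held items.
; A self-repeating delayed event sphere-traces from the camera, caching the BPI_Item actor in view and showing a pickup prompt.
; Pickup attaches that actor to the hand and records it in BPCBelt, while input keys send use, alternate-use and drop messages.
; Belt slot switching destroys the held actor and spawns the selected slot's stored class.
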(event `self.ReceiveBeginPlay`
  ; Begin Play
  (bind _asbp_first_person_character (cast `/Game/FirstPerson/Blueprints/BP_FirstPersonCharacter` (`self.GetOwner`)))
  (set `self.Player` _asbp_first_person_character)
  (set `self.First Person Camera` (`/Game/FirstPerson/Blueprints/BP_FirstPersonCharacter.FirstPersonCamera` _asbp_first_person_character))
  (`self.Try to interact`)
  (`self.SwapItem` 0))

(event `UpdateHeldItem`
  (params (`Newly Changed Slot` :type Integer)))

(event `OnSlotUpdated_Event`
  (params (UpdatedSlotIndex :type Integer)))

(event `Key|LeftMouseButton`
  (params (Key :type "Key Structure"))
  (:`Pressed`
    (`KismetSystemLibrary.PrintText` "Boop")
    (`self.Try to interact`)
    (if true
      (`KismetSystemLibrary.PrintString` "Killing Door"))))

(event `Try to interact`
  (bind _first_person_camera (`self.First Person Camera`))
  (bind _returnvalue (`SceneComponent.K2_GetComponentLocation` _first_person_camera))
  ; Looking
  (`KismetSystemLibrary.Delay` (`self.InteractINterval`))
  (bind (_outhit _returnvalue_2) (`KismetSystemLibrary.SphereTraceSingle` :`Start` _returnvalue :`End` (+ _returnvalue (* (`SceneComponent.GetForwardVector` _first_person_camera) (`self.Look Distancce`))) :`Radius` 20.0 :`TraceChannel` "TraceTypeQuery1" :`DrawDebugType` "ForDuration" :`TraceColor` (struct :`R` 1.0 :`G` 0.031817 :`B` 0.076594 :`A` 1.0) :`TraceHitColor` (struct :`R` 0.205778 :`G` 1.0 :`B` 0.193348 :`A` 1.0) :`DrawTime` 1.0))
  (if _returnvalue_2
    (bind (_bblockinghit _binitialoverlap _time _distance _location _impactpoint _normal _impactnormal _physmat _hitactor) (`GameplayStatics.BreakHitResult` _outhit))
    (if (`KismetSystemLibrary.DoesImplementInterface` _hitactor "/Game/Blueprints/BPI_Item.BPI_Item_C")
      (set `self.LastTouchedItem` _hitactor)
      (`KismetSystemLibrary.PrintText` (`|FormatText` "Press E to pick up {name}" (`KismetSystemLibrary.GetDisplayName` _hitactor)))
      (else
        (set `self.LastTouchedItem` null)))
    (else
      (set `self.LastTouchedItem` null)))
  (`self.Try to interact`))

(event `Try To Pick Up`
  (bind _player (`self.Player`))
  (`self.HeldItem`
    (:`then`)
    (:`else`
      (bind _lasttoucheditem (`self.LastTouchedItem`)
        (:`then`
          (bind _itemtype (message `/Game/Blueprints/BPI_Item.PickUp` _lasttoucheditem self))
          (`Actor.K2_AttachToComponent` _lasttoucheditem (`/Game/FirstPerson/Blueprints/BP_FirstPersonCharacter.Handhold Point` (`self.Player`)) "None" "SnapToTarget" "SnapToTarget" "KeepRelative" true)
          (bind _output_get (set `self.HeldItem` _lasttoucheditem))
          (`/Game/Blueprints/BPC_Inventory1.Setslot` (`/Game/FirstPerson/Blueprints/BP_FirstPersonCharacter.BPC_Belt` _player) (`self.Active slot`) _itemtype)
          (`Actor.SetActorEnableCollision` _output_get false)
          (`/Game/Inventory/UI/WBP_InventoryGrid.RefreshGrid` (`/Game/Inventory/UI/WBP_belt.WBP_InventoryGrid` (`/Game/FirstPerson/Blueprints/BP_FirstPersonCharacter.Belt Widget` _player))))
        (:`else`
          (`KismetSystemLibrary.PrintText` "we aren't looking at anythgin"))))))

(event `Key|E`
  (params (Key :type "Key Structure"))
  (:`Pressed`
    (`self.Try To Pick Up`)))

(event `Try to use`
  (bind _helditem (`self.HeldItem`)
    (:`then`
      (message `/Game/Blueprints/BPI_Item.Use` _helditem))
    (:`else`
      (`KismetSystemLibrary.PrintText` "We aren't holding anything" :!label _label))))

(event `Key|LeftMouseButton`
  (params (Key :type "Key Structure"))
  (:`Pressed`
    (`KismetSystemLibrary.PrintText` "Trying to use")
    (`self.Try to use`)))

(event `Key|Q`
  (params (Key :type "Key Structure"))
  (:`Pressed`
    (`self.Try to drop`)))

(event `Try to drop`
  (bind _helditem (`self.HeldItem`)
    (:`then`
      (`Actor.SetActorEnableCollision` _helditem true)
      (message `/Game/Blueprints/BPI_Item.Drop` _helditem)
      (`KismetSystemLibrary.Delay` 0.2))
    (:`else`
      (goto _label))))

(event `Key|C`
  (params (Key :type "Key Structure"))
  (:`Pressed`
    (`self.AlternateUse`)))

(event `/Game/Blueprints/BPI_Item.AlternateUse`
  (bind _helditem (`self.HeldItem`)
    (:`then`
      (`Actor.SetActorEnableCollision` _helditem true)
      (message `/Game/Blueprints/BPI_Item.AlternateUse` _helditem))
    (:`else`
      (goto _label))))

(event `Key|One`
  (params (Key :type "Key Structure"))
  ;[0.15 0.04649 0.1087 0.5] SwapItemINBelt
  (:`Pressed`
    (`self.SwapItem` 0)))

(event `Key|Two`
  (params (Key :type "Key Structure"))
  ;[0.15 0.04649 0.1087 0.5] SwapItemINBelt
  (:`Pressed`
    (`self.SwapItem` 1)))

(event `Key|Three`
  (params (Key :type "Key Structure"))
  ;[0.15 0.04649 0.1087 0.5] SwapItemINBelt
  (:`Pressed`
    (`self.SwapItem` 2)))

(event `SwapItem`
  (params (`New Slot index` :type Integer))
  (bind _handhold_point (`/Game/FirstPerson/Blueprints/BP_FirstPersonCharacter.Handhold Point` (`self.Player`)))
  (bind (_name _description _uiimage _actorbp _autopickupable _enum) (break `/Game/Blueprints/S_Item` (`/Game/Blueprints/BPC_Inventory1.GetSlot` (`/Game/FirstPerson/Blueprints/BP_FirstPersonCharacter.BPC_Belt` (`self.Player`)) `New Slot index`)))
  ;[0.15 0.04649 0.1087 0.5] SwapItemINBelt
  (if (== (`self.Active slot`) `New Slot index`)
    (`KismetSystemLibrary.PrintString` "Same Slot")
    (else
      (set `self.Active slot` `New Slot index`)
      (bind _helditem (`self.HeldItem`)
        (:`then`
          (`Actor.K2_DestroyActor` _helditem)
          (set `self.HeldItem` null))
        (:`else`
          _))
      (if (`|EnumEquality` _enum "NewEnumerator3")
        (`KismetSystemLibrary.PrintString` "Thats Empty")
        (else
          (bind _returnvalue (`|SpawnActorFromClass` _actorbp (`SceneComponent.GetRelativeTransform` _handhold_point) "Undefined" "MultiplyWithRoot" null null))
          (bind _output_get (set `self.HeldItem` _returnvalue))
          (`Actor.K2_AttachToComponent` _output_get _handhold_point "None" "KeepRelative" "KeepRelative" "KeepRelative" true)
          (message `/Game/Blueprints/BPI_Item.PickUp` (`self.HeldItem`) self))))))

(fn `PickUp`
  (params (Owner :type "/Game/Blueprints/BPC_Interact Object Reference")))