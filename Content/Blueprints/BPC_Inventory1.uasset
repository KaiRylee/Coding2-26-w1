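; BPC_Inventory1 is an inventory Blueprint that stores items as an array of enum values and resolves them to item data.
; GetSlot reads the enum at a slot and passes it to GetItemDetails, which scans every DT_Items row for the matching enum.
; Setslot writes a single array index, while SetInventory replaces the whole array and fires the OnSetInventory dispatcher.
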(fn `GetItemDetails`
  (params (`Requested Items` :type "/Game/Inventory/UI/E_Item Enum" :default "NewEnumerator0"))
  (returns (`Item Details` :type "/Game/Blueprints/S_Item Structure"))
  (bind _outrownames (`DataTableFunctionLibrary.GetDataTableRowNames` "/Game/Blueprints/DataTables/DT_Items.DT_Items"))
  (for _array_element _outrownames
    (bind _returnvalue (`|GetDataTableRow` "/Game/Blueprints/DataTables/DT_Items.DT_Items" _array_element)
      (:`then`
        (if (`|EnumEquality` (`.Enum_17_2AC826B3429E7D982CF0248466410A2E` (break `/Game/Blueprints/S_Item` _returnvalue)) `Requested Items`)
          (return _returnvalue))))))

(fn `GetSlot`
  (params (`Requested Slot` :type Integer))
  (returns (`Item Details` :type "/Game/Blueprints/S_Item Structure"))
  (bind _item_details (`self.GetItemDetails` (`|GetArrayItem` (`self.EnumInventory`) `Requested Slot`)))
  (return _item_details))

(fn `SetInventory`
  (params (EnumInv :type "Array of /Game/Inventory/UI/E_Item Enum"))
  (set `self.EnumInventory` EnumInv)
  (`self.OnSetInventory`))

(fn `Setslot`
  (params (Index :type Integer) (itemDetails :type "/Game/Inventory/UI/E_Item Enum" :default "NewEnumerator0"))
  (`KismetArrayLibrary.Array_Set` (`self.EnumInventory`) Index itemDetails))