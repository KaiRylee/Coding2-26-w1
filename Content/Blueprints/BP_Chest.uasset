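; Chest actor that opens when the first-person character enters its sphere and closes when they leave.
; OpenChest plays or reverses the Open timeline, which pitches the Hinge through a lerp.
; The timeline's Finished output shows the character's inventory and the chest menu widget created at BeginPlay, then prints the first item's name after a delay.
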(event `self.ReceiveBeginPlay`
  (bind _returnvalue (`|CreateWidget` "/Game/Inventory/UI/WBP_ChestMenu.WBP_ChestMenu_C" null (`self.Inventory`) (`self.BPC_Inventory1`)))
  (set `self.ChestMenu` _returnvalue))

(event `self.Sphere.OnComponentBeginOverlap`
  (params (OverlappedComponent :type "PrimitiveComponent Object Reference") (OtherActor :type "Actor Object Reference") (OtherComp :type "PrimitiveComponent Object Reference") (OtherBodyIndex :type Integer) (bFromSweep :type Boolean) (SweepResult :type "HitResult Structure (by ref)"))
  (bind _asbp_first_person_character (cast `/Game/FirstPerson/Blueprints/BP_FirstPersonCharacter` OtherActor))
  (`self.OpenChest` false))

(event `OpenChest`
  (params (Reverse :type Boolean))
  (if Reverse
    (bind (_direction _newtrack_0) (`Timeline|Open` :!via `Reverse` :!label _label)
      (:`Update`
        (`SceneComponent.K2_SetRelativeRotation` (`self.Hinge`) (`KismetMathLibrary.MakeRotator` 0.0 (`KismetMathLibrary.Lerp` 0.0 70.0 _newtrack_0)) false false))
      (:`Finished`
        (`/Game/FirstPerson/Blueprints/BP_FirstPersonCharacter.Show Inventory` (stale `self.Sphere.OnComponentBeginOverlap` _asbp_first_person_character))
        (`UserWidget.AddToViewport` (`self.ChestMenu`) 0)
        (`KismetSystemLibrary.Delay` 5.0)
        (`KismetSystemLibrary.PrintText` (`|FormatText` "First item in chest is a {name}" (`.Name_8_57A14A3348DA86656DB0F78DB7280B83` (break `/Game/Blueprints/S_Item` (`|GetArrayItem` (`self.Inventory`))))))))
    (else
      (goto _label))))

(event `self.Sphere.OnComponentEndOverlap`
  (params (OverlappedComponent :type "PrimitiveComponent Object Reference") (OtherActor :type "Actor Object Reference") (OtherComp :type "PrimitiveComponent Object Reference") (OtherBodyIndex :type Integer))
  (cast `/Game/FirstPerson/Blueprints/BP_FirstPersonCharacter` OtherActor)
  (`self.OpenChest` true))

(fn `UserConstructionScript`)