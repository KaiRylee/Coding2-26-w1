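; Player stats component that tracks health, stamina and mana and creates the WBP_Playerstats HUD widget on BeginPlay.
; Health packs min, max and current into one vector; stamina and mana bars are only initialized, straight from their Z values.
; ChangeHealth adds an unclamped delta, updates the bar and prints a death message.
; SetHealth treats -1 as a sentinel, but as wired only writes health and its bar when both min and max are -1.
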(event `self.ReceiveBeginPlay`
  (bind (_health_x _health_y _health_z) (`KismetMathLibrary.BreakVector` (`self.Health`)))
  (bind (_stamina_x _stamina_y _stamina_z) (`KismetMathLibrary.BreakVector` (`self.Stamina`)))
  (bind (_mana_x _mana_y _mana_z) (`KismetMathLibrary.BreakVector` (`self.Mana`)))
  (`|ExecutionSequence`
    (:`then_0`
      (bind _returnvalue (`|CreateWidget` "/Game/Inventory/UI/WBP_Playerstats.WBP_Playerstats_C"))
      (bind _output_get (set `self.StatsWidget` _returnvalue))
      (`UserWidget.AddToViewport` _output_get 0))
    (:`then_1`
      (`self.SetHealth` _health_x _health_y _health_z)
      (`ProgressBar.SetPercent` (`/Game/Inventory/UI/WBP_Playerstats.StaminaBar` (`self.StatsWidget`)) _stamina_z)
      (`ProgressBar.SetPercent` (`/Game/Inventory/UI/WBP_Playerstats.ManaBar` (`self.StatsWidget`)) _mana_z))))

(fn `ChangeHealth`
  (params (ByAmount :type "Float (double-precision)"))
  (bind (_health_x _health_y _health_z) (`KismetMathLibrary.BreakVector` (`self.Health`)))
  (bind (_health_x_2 _health_y_2 _health_z_2) (`KismetMathLibrary.BreakVector` (`self.Health`)))
  (bind _returnvalue (+ _health_z ByAmount))
  (set `self.Health` (`KismetMathLibrary.MakeVector` _health_x _health_y _returnvalue))
  (`ProgressBar.SetPercent` (`/Game/Inventory/UI/WBP_Playerstats.HealthBar` (`self.StatsWidget`)) (/ _health_z_2 (- _health_y_2 _health_x_2)))
  (if (<= _returnvalue 0.0)
    (`KismetSystemLibrary.PrintText` "Player Is Dead")))

(fn `SetHealth`
  (params (`Health X` :type "Float (double-precision)") (`Health Y` :type "Float (double-precision)") (`Health Z` :type "Float (double-precision)"))
  (locals (`Min Health` :type "Float (double-precision)") (`Max Health` :type "Float (double-precision)") (`Current Health` :type "Float (double-precision)"))
  (bind (_health_x _health_y _health_z) (`KismetMathLibrary.BreakVector` (`self.Health`)))
  (set `local.Min Health` (`local.Health X`))
  (set `local.Max Health` (`local.Health Y`))
  (set `local.Current Health` (`local.Health Z`))
  (if (!= `Health X` -1.0)
    (set `local.Min Health` `Health X`)
    (elif (!= `Health Y` -1.0)
      (set `local.Max Health` `Health Y`)
      (else
        (if true
          (set `local.Current Health` `Health Z`))
        (set `self.Health` (`KismetMathLibrary.MakeVector` (`local.Min Health`) (`local.Max Health`) (`local.Current Health`)))
        (`ProgressBar.SetPercent` (`/Game/Inventory/UI/WBP_Playerstats.HealthBar` (`self.StatsWidget`)) (/ _health_z (- _health_y _health_x)))))))