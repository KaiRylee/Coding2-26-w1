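; GM_SaveLoad is a game mode Blueprint that saves and restores the player's belt, inventory and last position through an SG_Player save object.
; On BeginPlay it loads the slot, pushing both item sets into BP_FirstPersonCharacter's components and moving its capsule unless the saved location is zero.
; Without an existing save, it creates a fresh save object.
; SavePlayer copies the passed-in state into that object, writes it to the slot and prints the result.
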(event `self.ReceiveBeginPlay`
  (`KismetSystemLibrary.PrintText` "GM_SaveLoad Is Running")
  (`self.LoadPlayer`))

(event `LoadPlayer`
  (bind _last_position (`/Game/Blueprints/SavingLoading/SG_Player.Last Position` (`self.PlayerSave`)))
  (bind _returnvalue (`GameplayStatics.DoesSaveGameExist` (`self.Slot Name`)))
  (if _returnvalue
    (bind _returnvalue_2 (`GameplayStatics.LoadGameFromSlot` (`self.Slot Name`)))
    (bind _assg_player (cast `/Game/Blueprints/SavingLoading/SG_Player` _returnvalue_2))
    (set `self.PlayerSave` _assg_player)
    (bind _asbp_first_person_character (cast `/Game/FirstPerson/Blueprints/BP_FirstPersonCharacter` (`GameplayStatics.GetPlayerCharacter` 0)))
    (`/Game/Blueprints/BPC_Inventory1.SetInventory` (`/Game/FirstPerson/Blueprints/BP_FirstPersonCharacter.BPC_Belt` _asbp_first_person_character) (`/Game/Blueprints/SavingLoading/SG_Player.Belt` (`self.PlayerSave`)))
    (`/Game/Blueprints/BPC_Inventory1.SetInventory` (`/Game/FirstPerson/Blueprints/BP_FirstPersonCharacter.BPC_Inventory1` _asbp_first_person_character) (`/Game/Blueprints/SavingLoading/SG_Player.Inventory` (`self.PlayerSave`)))
    (if (not (`KismetMathLibrary.EqualExactly_VectorVector` (.location _last_position)))
      (`SceneComponent.K2_SetWorldTransform` (`Character.CapsuleComponent` _asbp_first_person_character) _last_position false false))
    (else
      (bind _returnvalue_3 (`GameplayStatics.CreateSaveGameObject` "/Game/Blueprints/SavingLoading/SG_Player.SG_Player_C"))
      (set `self.PlayerSave` _returnvalue_3))))

(event `SavePlayer`
  (params (Belt :type "Array of /Game/Inventory/UI/E_Item Enum") (Inventory :type "Array of /Game/Inventory/UI/E_Item Enum") (InputPin :type "Transform Structure"))
  (bind _playersave (`self.PlayerSave`))
  (set `/Game/Blueprints/SavingLoading/SG_Player.Belt` Belt _playersave)
  (set `/Game/Blueprints/SavingLoading/SG_Player.Inventory` Inventory _playersave)
  (set `/Game/Blueprints/SavingLoading/SG_Player.Last Position` InputPin _playersave)
  (bind _returnvalue (`GameplayStatics.SaveGameToSlot` (`self.PlayerSave`) (`self.Slot Name`)))
  (if _returnvalue
    (`KismetSystemLibrary.PrintText` "Game Saved to Slot")
    (else
      (`KismetSystemLibrary.PrintText` "Could not save game to slot"))))

(fn `UserConstructionScript`)