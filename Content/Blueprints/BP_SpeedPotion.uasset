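; BP_SpeedPotion is a holdable potion item that can be picked up, drunk, thrown or dropped.
; PickUp stores the owner, disables Box collision and returns the item type.
; AlternateUse and Drop restore collision and physics, then apply a strong or gentle forward impulse.
; Use clears the owner's held item, destroys the potion and plays a gulp sound, with no speed effect applied here.
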(event `self.AlternateUse`
  (bind _box (`self.Box`))
  (bind _box_2 (`self.Box`))
  (`PrimitiveComponent.SetCollisionEnabled` _box "QueryAndPhysics")
  (`PrimitiveComponent.SetSimulatePhysics` _box_2 true)
  (`PrimitiveComponent.AddImpulse` _box_2 (* (`SceneComponent.GetForwardVector` _box) 500.0) "None" false))

(event `self.Use`
  (set `/Game/Blueprints/BPC_Interact.HeldItem` null (`self.Owner 0`))
  (`self.K2_DestroyActor` self)
  (`GameplayStatics.PlaySound2D` "/Game/Emma/Audio/Gulp.Gulp" 1.0 1.0 0.0 null null))

(event `self.Drop`
  (bind _box (`self.Box`))
  (bind _box_2 (`self.Box`))
  (`PrimitiveComponent.SetCollisionEnabled` _box "QueryAndPhysics")
  (`PrimitiveComponent.SetSimulatePhysics` _box_2 true)
  (`PrimitiveComponent.AddImpulse` _box_2 (* (`SceneComponent.GetForwardVector` _box) 10.0) "None" false))

(fn `PickUp`
  (params (Owner :type "/Game/Blueprints/BPC_Interact Object Reference"))
  (returns (ItemType :type "/Game/Inventory/UI/E_Item Enum"))
  (set `self.Owner 0` Owner)
  (`KismetSystemLibrary.PrintText` "Hello")
  (`PrimitiveComponent.SetCollisionEnabled` (`self.Box`) "NoCollision")
  (return (`self.ItemType`)))

(fn `UserConstructionScript`)