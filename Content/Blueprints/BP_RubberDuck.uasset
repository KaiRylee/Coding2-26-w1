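; BP_RubberDuck is a rubber duck item that can be picked up, used to play a squeak-style 2D sound, and dropped.
; PickUp stores the owner, turns off the Box collision, prints a debug greeting and returns the item type.
; Drop restores collision and physics with a gentle forward impulse, while an unnamed CustomEvent does the same with a much stronger, throw-like impulse.
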(event `self.Use`
  (`GameplayStatics.PlaySound2D` "/Game/Blueprints/Audio/SQ_Ducky.SQ_Ducky" 1.0 1.0 0.0 null null))

(event `CustomEvent`
  (bind _box (`self.Box`))
  (bind _box_2 (`self.Box`))
  (`PrimitiveComponent.SetCollisionEnabled` _box "QueryAndPhysics")
  (`PrimitiveComponent.SetSimulatePhysics` _box_2 true)
  (`PrimitiveComponent.AddImpulse` _box_2 (* (`SceneComponent.GetForwardVector` _box) 500.0) "None" false))

(event `self.Drop`
  (bind _box (`self.Box`))
  (bind _box_2 (`self.Box`))
  ; Drop
  (`PrimitiveComponent.SetCollisionEnabled` _box "QueryAndPhysics")
  (`PrimitiveComponent.SetSimulatePhysics` _box_2 true)
  (`PrimitiveComponent.AddImpulse` _box_2 (* (`SceneComponent.GetForwardVector` _box) 10.0) "None" false))

(fn `PickUp`
  (params (Owner :type "/Game/Blueprints/BPC_Interact Object Reference"))
  (returns (ItemType :type "/Game/Inventory/UI/E_Item Enum"))
  (set `self.Owner 0` Owner)
  (`KismetSystemLibrary.PrintText` "Hello")
  (`PrimitiveComponent.SetCollisionEnabled` (`self.Box`) "NoCollision")
  (return (`self.ItemType`)))

(fn `UserConstructionScript`)