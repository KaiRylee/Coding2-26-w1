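; Key item that a holder can pick up, drop, or use to open a BP_ClassDoor by destroying it.
; PickUp disables the box collision; Drop clears the holder's HeldItem, restores collision and physics, and launches the key forward with an impulse.
; Use runs a short forward Visibility trace from the box, destroying both door and key on a hit.
; AlternateUse only sets actor visibility, and both branches unhide it.
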(event `/Game/Blueprints/BPI_Item.PickUp`
  (params (Owner :type "/Game/Blueprints/BPC_Interact Object Reference"))
  (`KismetSystemLibrary.PrintText` "Hello")
  (`PrimitiveComponent.SetCollisionEnabled` (`self.Box`) "NoCollision"))

(event `/Game/Blueprints/BPI_Item.AlternateUse`
  (if (`self.New Hidden`)
    (`self.SetActorHiddenInGame` false)
    (else
      (`self.SetActorHiddenInGame` (`self.New Hidden`)))))

(event `/Game/Blueprints/BPI_Item.Use`
  (bind _box (`self.Box`))
  (bind _returnvalue (`SceneComponent.K2_GetComponentLocation` _box))
  (bind _outhit (`KismetSystemLibrary.LineTraceSingle` :`Start` _returnvalue :`End` (+ _returnvalue (* (`SceneComponent.GetForwardVector` _box) 300.0)) :`TraceChannel` "TraceTypeQuery1" :`DrawDebugType` "ForDuration"))
  (bind _asbp_class_door (cast `/Game/Blueprints/BP_ClassDoor` (`.HitActor` (`GameplayStatics.BreakHitResult` _outhit)))
    (:`then`
      (set `/Game/Blueprints/BPC_Interact.HeldItem` null (stale `/Game/Blueprints/BPI_Item.PickUp` Owner))
      (`self.K2_DestroyActor` _asbp_class_door)
      (`self.K2_DestroyActor` self))
    (:`CastFailed`
      (`KismetSystemLibrary.PrintText` "no"))))

(event `/Game/Blueprints/BPI_Item.Drop`
  (bind _box (`self.Box`))
  (bind _box_2 (`self.Box`))
  (set `/Game/Blueprints/BPC_Interact.HeldItem` null (stale `/Game/Blueprints/BPI_Item.PickUp` Owner))
  (`PrimitiveComponent.SetCollisionEnabled` _box "QueryAndPhysics")
  (`PrimitiveComponent.SetSimulatePhysics` _box_2 true)
  (`PrimitiveComponent.AddImpulse` _box_2 (* (`SceneComponent.GetForwardVector` _box) 1000.0) "None" false))

(fn `UserConstructionScript`)